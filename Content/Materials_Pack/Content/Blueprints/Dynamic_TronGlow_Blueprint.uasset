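; Dynamic_TronGlow_Blueprint gives itself a random glow colour through its construction script.
; It rolls independent red, green and blue values and creates a dynamic material instance from the Dymanic_TronGlow material.
; The random colour feeds that instance's "Glow Colour" parameter, and the instance is applied to material slot 0.
; Because this runs at construction, the colour re-rolls whenever the script reruns.
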(fn `UserConstructionScript`
  (bind _output_get (set `self.Red` (`KismetMathLibrary.RandomFloatInRange` 0.0 1.0)))
  (bind _output_get_2 (set `self.Green` (`KismetMathLibrary.RandomFloatInRange` 0.0 1.0)))
  (bind _output_get_3 (set `self.Blue` (`KismetMathLibrary.RandomFloatInRange` 0.0 1.0)))
  (bind _returnvalue (`KismetMaterialLibrary.CreateDynamicMaterialInstance` "/Game/Materials/Dymanic_TronGlow.Dymanic_TronGlow"))
  (set `self.NewMaterial` _returnvalue)
  (`MaterialInstanceDynamic.SetVectorParameterValue` _returnvalue "Glow Colour" (make `Object.LinearColor` _output_get _output_get_2 _output_get_3 1.0))
  (`PrimitiveComponent.SetMaterial` 0 (`self.NewMaterial`)))